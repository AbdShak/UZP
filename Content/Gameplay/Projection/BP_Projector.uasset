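; Perspective-puzzle projector that paints a hidden target actor onto scenery and restores it when the player's camera matches the capture viewpoint.
; Scene captures render the target's color and mask into render targets.
; When active, box traces through distance-sorted ProjectionOn actors spawn M_Projection decals on I_Test hits, each with an extra capture mask of nearer actors.
; Alignment unhides the target, enables collision and static-mesh physics, then destroys the projector.
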(event `Test`
  (bind _projectiontarget (`self.ProjectionTarget`))
  (`KismetSystemLibrary.Delay` 0.5)
  (`self.SetActorHiddenInGame` (`self.ProjectionTarget`) false)
  (`self.ProjectItem` :!label _label)
  (`KismetSystemLibrary.Delay` 0.1)
  (`self.SetActorHiddenInGame` _projectiontarget true)
  (`self.SetActorEnableCollision` _projectiontarget false))

(event `self.ReceiveBeginPlay`
  (`KismetSystemLibrary.PrintString` (`KismetSystemLibrary.GetDisplayName` self))
  (goto _label))

(event `self.ReceiveTick`
  (params (DeltaSeconds :type "Float (single-precision)"))
  (bind _newvar (`self.NewVar`))
  (if (`self.IsPlayerInPosition?`)
    (`self.FreeObject`)
    (`/Engine/EditorBlueprintResources/StandardMacros.IsValid` _newvar
      (:`Is Valid`
        (`self.Test` _newvar)))))

(fn `BoxTraceInfo`
  (returns (Start :type "Vector Structure") (End :type "Vector Structure") (Size :type "Vector Structure") (Rotation :type "Rotator Structure"))
  (bind _returnvalue (`self.K2_GetActorLocation`))
  (bind _scenecapturecomponent2d (`self.SceneCaptureComponent2D`))
  (return _returnvalue (+ _returnvalue (* (`SceneComponent.GetForwardVector` _scenecapturecomponent2d) 5000.0)) (200.0 200.0 200.0) (`SceneComponent.K2_GetComponentRotation` _scenecapturecomponent2d)))

(fn `FreeObject`
  (bind _projectiontarget (`self.ProjectionTarget`))
  (`self.SetActorHiddenInGame` _projectiontarget false)
  (`self.SetActorEnableCollision` _projectiontarget true)
  (bind _asstatic_mesh_actor (cast `StaticMeshActor` _projectiontarget)
    (:`then`
      (`PrimitiveComponent.SetSimulatePhysics` (`StaticMeshActor.StaticMeshComponent` _asstatic_mesh_actor) true)
      (`self.K2_DestroyActor`))
    (:`CastFailed`
      (`self.K2_DestroyActor`))))

(fn `IsPlayerInPosition?`
  (returns (NewParam :type Boolean))
  (bind _returnvalue (`GameplayStatics.GetPlayerCameraManager` 0))
  (bind _scenecapturecomponent2d (`self.SceneCaptureComponent2D`))
  (if (and (== (`SceneComponent.K2_GetComponentLocation` _scenecapturecomponent2d) (`self.K2_GetActorLocation` _returnvalue) :`ErrorTolerance` 20.0) (== (`SceneComponent.K2_GetComponentRotation` _scenecapturecomponent2d) (`self.K2_GetActorRotation` _returnvalue) :`ErrorTolerance` 5.0))
    (return true)))

(fn `ProjectItem`
  (bind _scenecapturecomponent2d (`self.SceneCaptureComponent2D`))
  (bind _scenecapturecomponent2d_2 (`self.SceneCaptureComponent2D`))
  (bind _mask (`self.Mask`))
  (bind _showonlyactors (`SceneCaptureComponent.ShowOnlyActors` (`self.Mask`)))
  (bind _showonlyactors_2 (`SceneCaptureComponent.ShowOnlyActors` (`self.SceneCaptureComponent2D`)))
  (`KismetSystemLibrary.PrintString` "Hello")
  (`SceneComponent.K2_SetWorldRotation` _scenecapturecomponent2d (`KismetMathLibrary.FindLookAtRotation` (`SceneComponent.K2_GetComponentLocation` _scenecapturecomponent2d) (`self.K2_GetActorLocation` (`self.ProjectionTarget`))) false false)
  (`SceneComponent.K2_SetWorldRotation` (`self.Mask`) (`KismetMathLibrary.FindLookAtRotation` (`SceneComponent.K2_GetComponentLocation` _scenecapturecomponent2d) (`self.K2_GetActorLocation` (`self.ProjectionTarget`))) false false)
  (`KismetArrayLibrary.Array_Clear` _showonlyactors_2)
  (`KismetArrayLibrary.Array_Add` _showonlyactors_2 (`self.ProjectionTarget`))
  (`KismetArrayLibrary.Array_Clear` _showonlyactors)
  (`KismetArrayLibrary.Array_Add` _showonlyactors (`self.ProjectionTarget`))
  (`|ExecutionSequence`
    (:`then_0`
      (bind _returnvalue (`KismetRenderingLibrary.CreateRenderTarget2D` 2048 2048))
      (set `SceneCaptureComponent2D.TextureTarget` _returnvalue _scenecapturecomponent2d_2)
      (`SceneCaptureComponent2D.CaptureScene` _scenecapturecomponent2d_2))
    (:`then_1`
      (bind _returnvalue_2 (`KismetRenderingLibrary.CreateRenderTarget2D` 1024 1024))
      (set `SceneCaptureComponent2D.TextureTarget` _returnvalue_2 _mask)
      (`SceneCaptureComponent2D.CaptureScene` _mask))
    (:`then_2`
      (`self.SortProjectedOnTargets`))
    (:`then_3`
      (`self.TraceProjection`))))

(fn `SortProjectedOnTargets`
  (locals (`L-IndexA` :type Integer) (`L-ActorA` :type "Actor Object Reference") (`L-IndexB` :type Integer) (`L-ActorB` :type "Actor Object Reference"))
  (for _index (range (+ (`KismetArrayLibrary.Array_LastIndex` (`self.ProjectionOn`)) 1))
    (set `local.L-IndexA` _index)
    (set `local.L-ActorA` (`|GetArrayItem` (`self.ProjectionOn`) (`local.L-IndexA`)))
    (for _index_2 (range (`local.L-IndexA`) (+ (`KismetArrayLibrary.Array_LastIndex` (`self.ProjectionOn`)) 1))
      (set `local.L-IndexB` _index_2)
      (set `local.L-ActorB` (`|GetArrayItem` (`self.ProjectionOn`) (`local.L-IndexB`)))
      (if (< (`self.GetDistanceTo` (`local.L-ActorB`)) (`self.GetDistanceTo` (`local.L-ActorA`)))
        (`KismetArrayLibrary.Array_Swap` (`self.ProjectionOn`) (`local.L-IndexA`) (`local.L-IndexB`))))))

(fn `TraceProjection`
  (locals (IgnoreActors :type "Array of Actor Object Reference") (ShowOnly :type "Array of Actor Object Reference") (CurrentTarget :type "Actor Object Reference") (`L-Decal` :type "DecalComponent Object Reference"))
  (bind (_start _end _size _rotation) (`self.BoxTraceInfo`))
  (bind (_start_2 _end_2 _size_2 _rotation_2) (`self.BoxTraceInfo`))
  (bind _currenttarget (`local.CurrentTarget`))
  (if (`self.bActive?`)
    (`|ExecutionSequence`
      (:`then_0`
        (bind _outhits (`KismetSystemLibrary.BoxTraceMulti` _start _end _size _rotation "TraceTypeQuery1" false (`self.ProjectionOn`) "ForDuration" true (struct :`B` 1.0 :`A` 1.0) (struct :`R` 1.0 :`G` 1.0 :`A` 1.0) 0.0))
        (for _array_element _outhits
          (bind (_bblockinghit _binitialoverlap _time _distance _location _impactpoint _normal _impactnormal _physmat _hitactor) (`GameplayStatics.BreakHitResult` _array_element))
          (`KismetArrayLibrary.Array_AddUnique` (`local.IgnoreActors`) _hitactor)
          (`KismetSystemLibrary.PrintString` (`KismetSystemLibrary.GetDisplayName` _hitactor) true true (struct :`R` 1.0 :`B` 0.177939 :`A` 1.0) 44.0))
        (`KismetArrayLibrary.Array_Add` (`local.IgnoreActors`) (`self.ProjectionTarget`))
        (`KismetArrayLibrary.Array_Append` (`local.IgnoreActors`) (`self.ActorsToIgnore`))
        (for _array_element_2 (`self.ProjectionOn`)
          (bind _output_get (set `local.CurrentTarget` _array_element_2))
          (bind _outhit (`KismetSystemLibrary.BoxTraceSingle` _start_2 _end_2 _size_2 _rotation_2 "TraceTypeQuery1" false (`local.IgnoreActors`) "None" true (struct :`R` 1.0 :`A` 1.0) (struct :`G` 1.0 :`A` 1.0) 20.0))
          (bind (_bblockinghit_2 _binitialoverlap_2 _time_2 _distance_2 _location_2 _impactpoint_2 _normal_2 _impactnormal_2 _physmat_2 _hitactor_2 _hitcomponent _hitbonename _bonename _hititem _elementindex _faceindex _tracestart _traceend) (`GameplayStatics.BreakHitResult` _outhit))
          (`KismetSystemLibrary.PrintString` (`KismetSystemLibrary.GetDisplayName` _hitactor_2) true true (struct :`G` 0.66 :`B` 1.0 :`A` 1.0) 44.0)
          (`|ExecutionSequence`
            (:`then_0`
              (if (`KismetSystemLibrary.DoesImplementInterface` _hitactor_2 "/Game/Gameplay/Interfaces/I_Test.I_Test_C")
                (bind _asstatic_mesh_component (cast `StaticMeshComponent` _hitcomponent))
                (bind _returnvalue (`self.GetTransform` (`ActorComponent.GetOwner` _asstatic_mesh_component)))
                (bind (_min _max) (`StaticMeshComponent.GetLocalBounds` _asstatic_mesh_component))
                (bind _returnvalue_2 (`AddComponent|NODE_AddDecalComponent-0` :`bManualAttachment` true :`RelativeTransform` (`KismetMathLibrary.MakeTransform` (+ (* (`KismetMathLibrary.Normal` (- _tracestart _traceend)) 5.0) (/ (+ (`KismetMathLibrary.TransformLocation` _returnvalue _min) (`KismetMathLibrary.TransformLocation` _returnvalue _max)) 2.0)) (`SceneComponent.K2_GetComponentRotation` _asstatic_mesh_component))))
                (bind _output_get_2 (set `local.L-Decal` _returnvalue_2))
                (`SceneComponent.SetWorldScale3D` _output_get_2 (`KismetMathLibrary.MakeVector` (- (.x (+ (* (`SceneComponent.K2_GetComponentScale` _asstatic_mesh_component) _max) 5.0)) (.x (`self.AdjustDecalPosition`))) (- (.y (+ (* (`SceneComponent.K2_GetComponentScale` _asstatic_mesh_component) _max) 5.0)) (.y (`self.AdjustDecalPosition`))) (- (.z (+ (* (`SceneComponent.K2_GetComponentScale` _asstatic_mesh_component) _max) 5.0)) (.z (`self.AdjustDecalPosition`)))))
                (bind _returnvalue_3 (`KismetRenderingLibrary.CreateRenderTarget2D` 2048 2048))
                (bind _returnvalue_4 (`AddComponent|NODE_AddSceneCaptureComponent2D-0` :`RelativeTransform` (`SceneComponent.GetRelativeTransform` (`self.SceneCaptureComponent2D`))))
                (set `SceneCaptureComponent2D.TextureTarget` _returnvalue_3 _returnvalue_4)
                (`KismetArrayLibrary.Array_Append` (`SceneCaptureComponent.ShowOnlyActors` _returnvalue_4) (`local.ShowOnly`))
                (`SceneCaptureComponent2D.CaptureScene` _returnvalue_4)
                (bind _returnvalue_5 (`KismetMaterialLibrary.CreateDynamicMaterialInstance` "/Game/Gameplay/Projection/M_Projection.M_Projection"))
                (`DecalComponent.SetDecalMaterial` (`local.L-Decal`) _returnvalue_5)
                (`self.UpdateMaterialParameters` _returnvalue_5 _returnvalue_3)))
            (:`then_1`
              (`KismetArrayLibrary.Array_Add` (`local.ShowOnly`) _currenttarget)
              (`KismetArrayLibrary.Array_Add` (`local.IgnoreActors`) _currenttarget))))))))

(fn `UpdateMaterialParameters`
  (params (Material :type "MaterialInstanceDynamic Object Reference") (Texture :type "TextureRenderTarget2D Object Reference"))
  (bind _scenecapturecomponent2d (`self.SceneCaptureComponent2D`))
  (bind _material (`local.Material`))
  (`MaterialInstanceDynamic.SetVectorParameterValue` _material "Location" (`KismetMathLibrary.Conv_VectorToLinearColor` (`SceneComponent.K2_GetComponentLocation` _scenecapturecomponent2d)))
  (`MaterialInstanceDynamic.SetVectorParameterValue` _material "RightVector" (`KismetMathLibrary.Conv_VectorToLinearColor` (`SceneComponent.GetRightVector` _scenecapturecomponent2d)))
  (`MaterialInstanceDynamic.SetVectorParameterValue` _material "UpVector" (`KismetMathLibrary.Conv_VectorToLinearColor` (`SceneComponent.GetUpVector` _scenecapturecomponent2d)))
  (`MaterialInstanceDynamic.SetVectorParameterValue` _material "ForwardVector" (`KismetMathLibrary.Conv_VectorToLinearColor` (`SceneComponent.GetForwardVector` _scenecapturecomponent2d)))
  (`MaterialInstanceDynamic.SetScalarParameterValue` _material "FOV" (`SceneCaptureComponent2D.FOVAngle` _scenecapturecomponent2d))
  (`MaterialInstanceDynamic.SetTextureParameterValue` _material "ProjectedActorTexture" (`SceneCaptureComponent2D.TextureTarget` (`self.Mask`)))
  (`MaterialInstanceDynamic.SetTextureParameterValue` _material "ProjectedTexture" (`SceneCaptureComponent2D.TextureTarget` _scenecapturecomponent2d))
  (`MaterialInstanceDynamic.SetTextureParameterValue` _material "ProjectedMask" (`local.Texture`)))

(fn `UserConstructionScript`
  (`KismetArrayLibrary.Array_Clear` (`SceneCaptureComponent.ShowOnlyActors` (`self.SceneCaptureComponent2D`)))
  (`KismetArrayLibrary.Array_Clear` (`SceneCaptureComponent.ShowOnlyActors` (`self.Mask`)))
  (`self.ProjectItem`))