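; Escalator actor that builds step meshes along a spline at Offset spacing in the construction script.
; Two motion approaches exist: a looping timeline lerping steps toward their neighbors, and a tick-style event advancing steps along the spline with wraparound.
; Their starting nodes are disconnected, so BeginPlay only plays a timeline that prints its value, leaving the steps static.
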(event `self.ReceiveBeginPlay`
  (bind (_direction _newtrack_0) (`Timeline|Timeline_1`)
    (:`Update`
      (`KismetSystemLibrary.PrintString` (`KismetStringLibrary.Conv_DoubleToString` _newtrack_0) true true (struct :`G` 0.66 :`B` 1.0 :`A` 1.0) 1000.0))))

(event `CustomEvent`
  (bind _steps (`self.Steps`))
  (bind _steps_2 (`self.Steps`))
  (set `self.Relative Location` (`SceneComponent.RelativeLocation` (`|GetArrayItem` (`self.Steps`))))
  (bind (_direction _newtrack_1) (`Timeline|Timeline` :!via `PlayFromStart`)
    (:`Update`
      (for (_array_element _array_index) _steps_2
        (if (!= (`KismetArrayLibrary.Array_LastIndex` _steps_2) _array_index)
          (bind _relativelocation (`SceneComponent.RelativeLocation` (`|GetArrayItem` _steps_2 _array_index)))
          (`SceneComponent.K2_SetRelativeLocation` _array_element (`KismetMathLibrary.VLerp` _relativelocation (`|GetArrayItem` (`self.Steps_0`) _array_index) _newtrack_1) false false)
          (else
            (`SceneComponent.K2_SetRelativeLocation` _array_element (`KismetMathLibrary.VLerp` _relativelocation (`self.Relative Location`) _newtrack_1) false false)))))
    (:`Finished`
      (`KismetArrayLibrary.Array_Clear` (`self.Steps_0`))
      (for (_ _array_index_2) _steps
        (if (!= (`KismetArrayLibrary.Array_LastIndex` _steps) _array_index_2)
          (`KismetArrayLibrary.Array_Add` (`self.Steps_0`) (`SceneComponent.RelativeLocation` (`|GetArrayItem` _steps (+ _array_index_2 1))))
          (else
            (`KismetArrayLibrary.Array_Add` (`self.Steps_0`) (`SceneComponent.RelativeLocation` (`|GetArrayItem` _steps))))))
      (`self.CustomEvent`))))

(event `CustomEvent_0`
  (bind _spline (`self.Spline`))
  (bind _returnvalue (`SplineComponent.GetSplineLength` _spline))
  (if (`KismetArrayLibrary.Array_IsValidIndex` (`self.Steps`))
    (bind _output_get (set `self.distance` (`KismetMathLibrary.FInterpTo_Constant` (`self.distance`) (`SplineComponent.GetSplineLength` (`self.Spline`)) (`GameplayStatics.GetWorldDeltaSeconds`) 75.0)))
    (`KismetSystemLibrary.PrintString` (`KismetStringLibrary.Conv_DoubleToString` _output_get))
    (for (_array_element _array_index) (`self.Steps`)
      (bind _returnvalue_2 (+ (`self.distance`) (* (`self.offset`) _array_index)))
      (`SceneComponent.K2_SetWorldLocation` _array_element (`SplineComponent.GetLocationAtDistanceAlongSpline` _spline (`KismetMathLibrary.SelectFloat` (- _returnvalue_2 _returnvalue) _returnvalue_2 (> _returnvalue_2 _returnvalue)) "World") false false))
    (if (`KismetMathLibrary.NearlyEqual_FloatFloat` (`self.distance`) (`SplineComponent.GetSplineLength` (`self.Spline`)) 0.01)
      (set `self.distance` 0.0))))

(fn `UserConstructionScript`
  (bind _offset (`self.offset`))
  (`KismetArrayLibrary.Array_Clear` (`self.Steps`))
  (for _index (range (+ (`KismetMathLibrary.FFloor` (/ (`SplineComponent.GetSplineLength` (`self.Spline`)) _offset)) 1))
    (bind _returnvalue (`AddComponent|NODE_AddStaticMeshComponent-0` :`RelativeTransform` (`KismetMathLibrary.MakeTransform` (`SplineComponent.GetLocationAtDistanceAlongSpline` (`self.Spline`) (`KismetMathLibrary.Conv_IntToDouble` (* _index _offset)) "Local") (struct :`Yaw` 90.0))))
    (`KismetArrayLibrary.Array_Add` (`self.Steps`) _returnvalue)))