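; BP_Object is an actor with a static mesh and a decal that can be detached into a loose physics object.
; The construction script applies a configurable decal material, and BeginPlay makes the mesh ignore WorldDynamic.
; Detach shows the mesh, makes it movable and simulated, hides the decal and blocks WorldDynamic.
; A flag exposed through IsDetached records the state, while the Hold_1 event is empty.
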(event `self.ReceiveBeginPlay`
  (`PrimitiveComponent.SetCollisionResponseToChannel` (`self.StaticMesh`) "ECC_WorldDynamic" "ECR_Ignore"))

(event `Hold_1`)

(event `/Game/Gameplay/Interfaces/I_Detachable.Detach`
  (bind _staticmesh (`self.StaticMesh`))
  (`SceneComponent.SetVisibility` _staticmesh true false)
  (`SceneComponent.SetMobility` _staticmesh "Movable")
  (`PrimitiveComponent.SetSimulatePhysics` _staticmesh true)
  (`SceneComponent.SetVisibility` (`self.Decal`) false false)
  (set `self.bDetached?` true)
  (`PrimitiveComponent.SetCollisionResponseToChannel` (`self.StaticMesh`) "ECC_WorldDynamic" "ECR_Block"))

(fn `IsDetached?`
  (returns (`IsDeached?` :type Boolean))
  (return (`self.bDetached?`)))

(fn `UserConstructionScript`
  (`DecalComponent.SetDecalMaterial` (`self.Decal`) (`self.New Decal Material`)))