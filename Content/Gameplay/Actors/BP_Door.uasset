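; BP_Door is a sliding door actor that opens when its Action event fires.
; BeginPlay stores the door mesh's world location, and Action plays a timeline that lerps the door from there to a fixed offset along the Arrow component's forward vector.
; The arrow sets the slide direction, and no reverse or closing logic is present.
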(event `self.ReceiveBeginPlay`
  (set `self.OrginalLocation` (`SceneComponent.K2_GetComponentLocation` (`self.Door`))))

(event `/Game/Gameplay/Interfaces/I_Interactable.Action`
  (bind _orginallocation (`self.OrginalLocation`))
  (bind (_direction _amount) (`Timeline|Timeline`)
    (:`Update`
      (`SceneComponent.K2_SetWorldLocation` (`self.Door`) (`KismetMathLibrary.VLerp` _orginallocation (+ _orginallocation (* (`SceneComponent.GetForwardVector` (`self.Arrow`)) 250.0)) _amount) false false))))

(fn `UserConstructionScript`)