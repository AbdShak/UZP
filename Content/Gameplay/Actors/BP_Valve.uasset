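; BP_Valve is a valve actor that, when its Action event fires, spins its mesh and slides a set of linked actors.
; Action caches the location of each entry in ActorsToMove, then plays a timeline from the start.
; The timeline lerps those actors 100 units along world X from the cached positions while incrementally yawing the mesh.
; On finish, it calls Test on the NewVar reference.
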(event `/Game/Gameplay/Interfaces/I_Interactable.Action`
  (bind _staticmesh1 (`self.StaticMesh1`))
  (bind _relativerotation (`SceneComponent.RelativeRotation` _staticmesh1))
  (`KismetArrayLibrary.Array_Clear` (`self.CurrentWallsLocations`))
  (for _array_element (`self.ActorsToMove`)
    (`KismetArrayLibrary.Array_Add` (`self.CurrentWallsLocations`) (`self.K2_GetActorLocation` _array_element)))
  (bind (_direction _newtrack_0) (`Timeline|Timeline` :!via `PlayFromStart`)
    (:`Update`
      (`SceneComponent.K2_SetRelativeRotation` _staticmesh1 (`KismetMathLibrary.RLerp` _relativerotation (`KismetMathLibrary.MakeRotator` (.roll _relativerotation) (.pitch _relativerotation) (+ (.yaw _relativerotation) 2.0)) _newtrack_0) false false)
      (for (_array_element_2 _array_index) (`self.ActorsToMove`)
        (bind _output (`|GetArrayItem` (`self.CurrentWallsLocations`) _array_index))
        (`self.K2_SetActorLocation` _array_element_2 (`KismetMathLibrary.VLerp` _output (+ _output (100.0 0.0 0.0)) _newtrack_0) false false)))
    (:`Finished`
      (`/Game/Gameplay/Projection/BP_Projector.Test` (`self.NewVar`)))))

(fn `UserConstructionScript`)